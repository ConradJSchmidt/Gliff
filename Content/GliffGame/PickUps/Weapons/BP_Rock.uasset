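; BP_Rock is a throwable rock weapon that damages BP_Bulls actors it hits.
; Thrown sets projectile velocity from player pawn and WeaponComponent velocities multiplied by pawn forward, then enables physics, collision, gravity and projectile movement.
; Any Sphere overlap deactivates projectile movement; after a short delay, a bull takes damage and the rock destroys itself, while other actors leave it in place.
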(event OnComponentBeginOverlap(Sphere)
  (params (OverlappedComponent :type Primitive%20Component%20Object%20Reference) (OtherActor :type Actor%20Object%20Reference) (OtherComp :type Primitive%20Component%20Object%20Reference) (OtherBodyIndex :type Integer) (bFromSweep :type Boolean) (SweepResult :type Hit%20Result%20Structure%20%28by%20ref%29))
  (bind _projectilemovement (Variables|Default|GetProjectileMovement))
  (if (Utilities|IsValid _projectilemovement)
    (Components|Activation|Deactivate _projectilemovement)
    (Utilities|FlowControl|Delay 0.2)
    (bind _asbp_bulls (Utilities|Casting|CastToBP_Bulls OtherActor))
    (Game|Damage|ApplyDamage _asbp_bulls 1e+02 0 0)
    (Actor|DestroyActor)))

(event EventThrown
  (bind _collisiongeneric (Variables|Default|GetCollisionGeneric))
  (Game|Components|ProjectileMovement|SetVelocityinLocalSpace (Variables|Default|GetProjectileMovement) (* (+ (Transformation|GetVelocity (Game|Player|GetPlayerPawn 0)) (Transformation|GetComponentVelocity (Variables|Default|GetWeaponComponent))) (Transformation|GetActorForwardVector (Game|Player|GetPlayerPawn 0))))
  (Physics|SetSimulatePhysics _collisiongeneric true)
  (Collision|SetCollisionEnabled _collisiongeneric "QueryAndPhysics")
  (Physics|SetEnableGravity _collisiongeneric true)
  (Components|Activation|Activate (Variables|Default|GetProjectileMovement) false))

(fn ConstructionScript)