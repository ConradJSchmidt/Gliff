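; BP_InHandWeapon is the weapon mesh held in the player's hand.
; Its construction script turns off physics and gravity on the mesh when it is equipped.
; CheckIfLastWeapon looks up the player's current weapon type in the weapon data table and hides the mesh when that row's ammo count is zero or less.
; The Thrown event is an empty stub.
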(event Custom|CheckIfLastWeapon
  (bind _asbp_gliff_player (Utilities|Casting|CastToBP_GliffPlayer (Game|Player|GetPlayerPawn 0)))
  (bind _returnvalue (Utilities|GetDataTableRow "/Game/GliffGame/PickUps/Weapons/WeaponDataTable.WeaponDataTable" (Utilities|Name|EnumtoName (Variables|/Game/GliffGame/SideScrollGame/BP_GliffPlayer.BP_GliffPlayer_C|GetCurrentWeaponType _asbp_gliff_player)))
    (:then
      (if (<= (.ammocount _returnvalue) 0.0)
        (Rendering|SetVisibility (Variables|Default|GetInHandWeapon) false false)))))

(event Custom|Thrown)

(fn ConstructionScript
  (bind _inhandweapon (Variables|Default|GetInHandWeapon))
  (if (Variables|Default|GetIsEquipped)
    (Physics|SetSimulatePhysics _inhandweapon false)
    (Physics|SetEnableGravity _inhandweapon false)))