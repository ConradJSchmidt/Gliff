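; BP_ThrownWeapon is an actor for a thrown weapon, built around a physics-driven ThrownWeapon component.
; Its construction script turns on physics simulation and gravity for that component.
; BeginPlay is empty, and unconnected leftover launch logic would show the component, set X velocity from player velocity and direction, reset rotation, and add an InitialVelocity impulse.
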(event EventBeginPlay)

(fn ConstructionScript
  (bind _thrownweapon (Variables|Default|GetThrownWeapon))
  (Physics|SetSimulatePhysics _thrownweapon true)
  (Physics|SetEnableGravity _thrownweapon true))