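; Boomerang weapon actor that flies out from the throw point, homes back to the player and damages BP_Bulls on overlap.
; Thrown swaps mesh visibility and plane-constrains ProjectileMovement in side-scroll mode.
; A Forward timeline drives a swept, height-clamped path including player velocity; a Return timeline lerps to the player's live location, then destroys it and calls CatchBoomerang.
; Bull hits deactivate the damage collider for a short cooldown.
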(event OnComponentBeginOverlap(DamageCollider)
  (params (OverlappedComponent :type Primitive%20Component%20Object%20Reference) (OtherActor :type Actor%20Object%20Reference) (OtherComp :type Primitive%20Component%20Object%20Reference) (OtherBodyIndex :type Integer) (bFromSweep :type Boolean) (SweepResult :type Hit%20Result%20Structure%20%28by%20ref%29))
  (bind _damagecollider (Variables|Default|GetDamageCollider))
  (Audio|PlaySoundatLocation "/Game/GliffGame/Audio/SFX/SPEAR_IMPACT_6_Cue.SPEAR_IMPACT_6_Cue" "0, 0, 0" "0, 0, 0" 1.0 1.0 0.0 0 0 0 0)
  (bind _asbp_bulls (Utilities|Casting|CastToBP_Bulls OtherActor))
  (Game|Damage|ApplyDamage _asbp_bulls 25.0 0 0)
  (Components|Activation|Deactivate _damagecollider)
  (Utilities|FlowControl|Delay 1.0)
  (Components|Activation|Activate _damagecollider true))

(event EventThrown
  (bind _returnvalue (Transformation|GetActorLocation))
  (bind _returnvalue_2 (Audio|SpawnSoundAttached "/Game/GliffGame/Audio/SFX/BOMERANG_Cue.BOMERANG_Cue" (Variables|Default|GetBoomerang3) "None" "0, 0, 0" "0, 0, 0" "KeepRelativeOffset" true 1.0 1.0 0.0 0 0))
  (Variables|Default|SetBoomerangSound _returnvalue_2)
  (bind _asbp_gliff_player (Utilities|Casting|CastToBP_GliffPlayer (Game|GetPlayerCharacter 0)))
  (Variables|Default|SetAs%20BP%20Gliff%20Player _asbp_gliff_player)
  (if (Variables|/Game/GliffGame/SideScrollGame/BP_GliffPlayer.BP_GliffPlayer_C|GetIsSideScroll _asbp_gliff_player)
    (Class|MovementComponent|SetPlaneConstraintEnabled (Variables|Default|GetProjectileMovement) true)
    (Class|MovementComponent|SetPlaneConstraintNormal (Variables|Default|GetProjectileMovement) "0.000000,1.000000,0.000000")
    (else
      (Class|MovementComponent|SetPlaneConstraintEnabled (Variables|Default|GetProjectileMovement) false)
      (Class|MovementComponent|SetPlaneConstraintNormal (Variables|Default|GetProjectileMovement) "0, 0, 0")))
  (Rendering|SetVisibility (Variables|Default|GetInHandWeapon) false false)
  (Rendering|SetVisibility (Variables|Default|GetBoomerang3) true false)
  (Variables|Default|SetFinalVelocity (+ (* (Transformation|GetActorForwardVector) "2900.000000,2900.000000,-200.000000") (Transformation|GetVelocity (Game|GetPlayerCharacter 0))))
  (Variables|Default|SetStartLocation (Transformation|GetActorLocation))
  (bind _alpha (Timeline|Forward PlayFromStart)
    (:Update
      (Transformation|SetActorLocation (+ (Variables|Default|GetStartLocation) (* (Variables|Default|GetFinalVelocity) _alpha)) true false)
      (Transformation|SetActorLocation (Math|Vector|MakeVector (.x _returnvalue) (.y _returnvalue) (Math|Float|Clamp(Float) 0.0 (+ (.z _returnvalue) 5e+01) (+ (.z (Transformation|GetActorLocation (Game|GetPlayerCharacter 0))) 3e+02))) true false))
    (:Finished
      (Variables|Default|SetFinalLocation (Transformation|GetActorLocation))
      (bind _alpha_2 (Timeline|Return PlayFromStart)
        (:Update
          (Transformation|SetActorLocation (Math|Vector|Lerp(Vector) (Variables|Default|GetFinalLocation) (Transformation|GetActorLocation (Game|GetPlayerCharacter 0)) _alpha_2) true false))
        (:Finished
          (Rendering|SetVisibility (Variables|Default|GetInHandWeapon) true false)
          (Rendering|SetVisibility (Variables|Default|GetBoomerang3) false false)
          (Actor|DestroyActor)
          (Audio|PlaySoundatLocation "/Game/GliffGame/Audio/SFX/CATCH_BOOMERANG_5_Cue.CATCH_BOOMERANG_5_Cue" "0, 0, 0" "0, 0, 0" 1.0 1.0 0.0 0 0 0 0)
          (Default|CatchBoomerang (Variables|Default|GetAs%20BP%20Gliff%20Player))
          (Utilities|IsValid (Variables|Default|GetBoomerangSound)
            (:Is%20Valid
              (Audio|Components|Audio|Stop (Variables|Default|GetBoomerangSound)))))))))

(fn ConstructionScript)