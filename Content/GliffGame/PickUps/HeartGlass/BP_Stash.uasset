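; BP_Stash is a one-shot pickup that adds to the player's HealthStash when BP_GliffPlayer overlaps FoodPickUp, then calls CheckHealthStash.
; TriggerFX plays a sound, spawns a burst particle system, hides the spike and skull meshes and disables spike and pickup collision.
; It reveals SMBurstA with a dynamic material created at BeginPlay, passing game time to AnimationControl to time the burst animation.
; The actor destroys itself after a short delay.
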(event OnComponentBeginOverlap(FoodPickUp)
  (params (OverlappedComponent :type Primitive%20Component%20Object%20Reference) (OtherActor :type Actor%20Object%20Reference) (OtherComp :type Primitive%20Component%20Object%20Reference) (OtherBodyIndex :type Integer) (bFromSweep :type Boolean) (SweepResult :type Hit%20Result%20Structure%20%28by%20ref%29))
  ;[0.15 0.15 0.15 0.5] AddHealthStash
  (bind _asbp_gliff_player (Utilities|Casting|CastToBP_GliffPlayer OtherActor))
  (Variables|/Game/GliffGame/SideScrollGame/BP_GliffPlayer.BP_GliffPlayer_C|SetHealthStash _asbp_gliff_player (+ (Variables|/Game/GliffGame/SideScrollGame/BP_GliffPlayer.BP_GliffPlayer_C|GetHealthStash _asbp_gliff_player) 10))
  (Default|CheckHealthStash _asbp_gliff_player)
  (CallFunction|TriggerFX))

(event Custom|TriggerFX
  (bind _dynamicmaterial (Variables|Default|GetDynamicMaterial))
  ;[0.15 0.15 0.15 0.5] TriggerFX
  (Audio|PlaySoundatLocation (Variables|Default|GetSound) "0, 0, 0" "0, 0, 0" 1.0 1.0 0.0 0 0 0 0)
  (Niagara|SpawnSystematLocation "/Game/GliffGame/VFX/Niagra/PS_BurstRed2.PS_BurstRed2" (Transformation|GetWorldLocation (Variables|Default|GetSM_BurstA)) "0, 0, 0" "2.000000,2.000000,2.000000")
  (Rendering|Material|SetMaterial (Variables|Default|GetSM_BurstA) 0 _dynamicmaterial)
  (Rendering|Material|SetScalarParameterValue _dynamicmaterial "AnimationControl" (Utilities|Time|GetGameTimeinSeconds) :!class /Script/Engine.MaterialInstanceDynamic)
  (Rendering|SetVisibility (Variables|Default|GetSM_BurstA) true false)
  (Rendering|SetVisibility (Variables|Default|GetSM_Spike) false false)
  (Collision|SetCollisionEnabled (Variables|Default|GetSM_Spike) "NoCollision")
  (Utilities|FlowControl|Delay 1.0)
  (Actor|DestroyActor))

(event EventBeginPlay
  ;[0.15 0.15 0.15 0.5] TriggerFX
  (bind _returnvalue (Rendering|Material|CreateDynamicMaterialInstance (Variables|Default|GetSM_BurstA) 0 "/Game/GliffGame/VFX/Materials/SPRITES/M_FlipBurstA_Inst.M_FlipBurstA_Inst" "None" :!class /Script/Engine.PrimitiveComponent))
  (Variables|Default|SetDynamicMaterial _returnvalue))

(fn ConstructionScript)