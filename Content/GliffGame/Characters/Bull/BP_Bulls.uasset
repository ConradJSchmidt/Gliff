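; Bull character that flees from the player when the player or another bull enters its proximity spheres.
; A looping timer drives movement away from the player, with dust and footstep sounds, until RunDistance is covered.
; Damage feeds BPHealthSystemComponent, playing launch-and-montage reactions before fleeing.
; Death triggers a poof, launches a physics skull from a spawned stash, destroys the actor and calls ApplyHealth on the player.
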(event OnComponentBeginOverlap(ProximitySphere2)
  (params (OverlappedComponent :type Primitive%20Component%20Object%20Reference) (OtherActor :type Actor%20Object%20Reference) (OtherComp :type Primitive%20Component%20Object%20Reference) (OtherBodyIndex :type Integer) (bFromSweep :type Boolean) (SweepResult :type Hit%20Result%20Structure%20%28by%20ref%29))
  ;[0.15 0.15 0.15 0.5] RunTriggers
  (bind _asbp_bulls (Utilities|Casting|CastToBP_Bulls OtherActor))
  (if (!= _asbp_bulls self)
    (CallFunction|OnBullIsScared)))

(event OnComponentBeginOverlap(ProximitySphere)
  (params (OverlappedComponent :type Primitive%20Component%20Object%20Reference) (OtherActor :type Actor%20Object%20Reference) (OtherComp :type Primitive%20Component%20Object%20Reference) (OtherBodyIndex :type Integer) (bFromSweep :type Boolean) (SweepResult :type Hit%20Result%20Structure%20%28by%20ref%29))
  ;[0.15 0.15 0.15 0.5] RunTriggers
  (Utilities|Casting|CastToBP_GliffPlayer OtherActor)
  (CallFunction|OnBullIsScared))

(event Custom|OnBullIsScared
  ;[0.15 0.15 0.15 0.5] RunAway
  (Components|Activation|Activate (Variables|Default|Getdust) false)
  (Variables|Default|SetStartLocation (Transformation|GetActorLocation))
  (Variables|Default|SetIsRunning true)
  (CallFunction|RunSound)
  (bind _returnvalue (Utilities|Time|SetTimerbyEvent (delegate Custom|BullRun) 0.01 true))
  (Variables|Default|SetTimerHandle _returnvalue))

(event Custom|BullRun
  ;[0.15 0.15 0.15 0.5] RunAway
  (Pawn|Input|AddMovementInput (* (Math|Vector|Normalize (- (Transformation|GetActorLocation (Game|Player|GetPlayerPawn 0)) (Transformation|GetActorLocation))) -0.2) 1.5 true)
  (if (>= (Math|Vector|VectorLength (- (Transformation|GetActorLocation) (Variables|Default|GetStartLocation))) (Variables|Default|GetRunDistance))
    (Utilities|Time|ClearandInvalidateTimerbyHandle (Variables|Default|GetTimerHandle))
    (Components|Movement|StopMovementImmediately (Variables|Character|GetCharacterMovement))
    (Components|Activation|Deactivate (Variables|Default|Getdust))
    (Variables|Default|SetIsRunning false)
    (CallFunction|RunSound)))

(event Custom|CowDeath
  ;[0.15 0.15 0.15 0.5] DammageAndDeath
  (if (Variables|Default|GetCowIsDead)
    (Audio|SpawnSoundatLocation "/Game/GliffGame/Audio/SFX/FEAST_POOF_DIAPPEARS.FEAST_POOF_DIAPPEARS" "0, 0, 0" "0, 0, 0" 1.0 1.0 0.0 0 0)
    (Collision|SetCollisionEnabled (Variables|Collision|GetCapsuleComponent) "NoCollision")
    (Rendering|SetVisibility (Variables|Default|GetLIGHTpOOF) true false)
    (Components|Activation|Activate (Variables|Default|GetPoof) false)
    (Rendering|SetVisibility (Variables|Character|GetMesh) false false)
    (CallFunction|SpawnPickUp)
    (Utilities|FlowControl|Delay 0.5)
    (Rendering|SetVisibility (Variables|Default|GetLIGHTpOOF) false true)
    (Utilities|FlowControl|Delay 1.5)
    (Actor|DestroyActor)
    (bind _asbp_gliff_player (Utilities|Casting|CastToBP_GliffPlayer (Game|GetPlayerCharacter 0)))
    (Default|ApplyHealth _asbp_gliff_player)))

(event Custom|SpawnPickUp
  ;[0.15 0.15 0.15 0.5] SpawnPickUp
  (if (not (Variables|Default|GetSkullHasSpawned))
    (bind _asbp_stash (Utilities|Casting|CastToBP_StashClass "/Game/GliffGame/VFX/SM/BP_Stash.BP_Stash_C"))
    (bind _returnvalue (Game|SpawnActorfromClass _asbp_stash (Transformation|GetActorTransform) "Undefined" "MultiplyWithRoot" 0 0))
    (Physics|SetEnableGravity (Variables|/Game/GliffGame/VFX/SM/BP_Stash.BP_Stash_C|GetSkull _returnvalue) true)
    (Physics|SetSimulatePhysics (Variables|/Game/GliffGame/VFX/SM/BP_Stash.BP_Stash_C|GetSkull _returnvalue) true)
    (Physics|AddImpulse (Variables|/Game/GliffGame/VFX/SM/BP_Stash.BP_Stash_C|GetSkull _returnvalue) "0.000000,0.000000,1000.000000" "None" true)
    (Variables|Default|SetSkullHasSpawned true)))

(event Custom|RunSound
  (if (Variables|Default|GetIsRunning)
    (Audio|PlaySoundatLocation "/Game/GliffGame/Audio/SFX/BULL_FEET_5_Cue.BULL_FEET_5_Cue" "0, 0, 0" "0, 0, 0" 1.0 1.0 0.0 0 0 0 0)
    (Utilities|FlowControl|Delay 0.5)
    ;[0.15 0.15 0.15 0.5] RunAway
    (Audio|PlaySoundatLocation "/Game/GliffGame/Audio/SFX/BULL_FEET_5_Cue.BULL_FEET_5_Cue" "0, 0, 0" "0, 0, 0" 1.0 1.0 0.0 0 0 0 0)
    (Utilities|FlowControl|Delay 0.5)
    (Audio|PlaySoundatLocation "/Game/GliffGame/Audio/SFX/BULL_FEET_5_Cue.BULL_FEET_5_Cue" "0, 0, 0" "0, 0, 0" 1.0 1.0 0.0 0 0 0 0)))

(event Game|Damage|EventAnyDamage
  (params (Damage :type Float%20%28single-precision%29) (DamageType :type Damage%20Type%20Object%20Reference) (InstigatedBy :type Controller%20Object%20Reference) (DamageCauser :type Actor%20Object%20Reference))
  (bind _mesh (Variables|Character|GetMesh))
  ;[0.15 0.15 0.15 0.5] DammageAndDeath
  (if (not (Variables|Default|GetCowIsDead))
    (Default|TookDamage (Variables|Default|GetBP_HealthSystem_Component) 0 Damage)
    (if (<= (Variables|/Game/GliffGame/SideScrollGame/Components/BP_HealthSystem_Component.BP_HealthSystem_Component_C|GetHealth (Variables|Default|GetBP_HealthSystem_Component)) 0.0)
      (Variables|Default|SetCowIsDead true)
      (CallFunction|CowDeath)
      (else
        (Character|LaunchCharacter "-100.000000,0.000000,450.000000" false false)
        (Animation|Montage|PlayMontage _mesh "/Game/GliffGame/Characters/Bull/Animation/AM_Bull_Hit_001.AM_Bull_Hit_001"
          (:OnBlendOut
            (Character|LaunchCharacter "50.000000,0.000000,550.000000" false false)
            (Animation|Montage|PlayMontage _mesh "/Game/GliffGame/Characters/Bull/Animation/AM_Bull_Turn_001.AM_Bull_Turn_001" 1.0 -1.0
              (:OnBlendOut
                (Character|LaunchCharacter "50.000000,0.000000,-100.000000" false false)
                (CallFunction|OnBullIsScared)
                (Animation|Montage|PlayMontage 0 "/Game/GliffGame/Characters/Bull/Animation/AM_Bull_Run_002.AM_Bull_Run_002")))))))))

(fn ConstructionScript)

(fn CheckRunDistance)