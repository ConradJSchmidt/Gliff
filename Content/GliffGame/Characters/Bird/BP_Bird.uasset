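; BP_Bird is a bird that flees along its Escape spline, driven by a timeline, when the player enters its trigger box.
; Hit-collider overlaps show explosion effects; an in-hand weapon also stops flight, drops the bird with physics and applies delayed damage through its health component.
; At zero health it destroys itself and calls BullApplyHealth on the player.
; A separate SpawnPickUp event, uncalled here, launches a one-time stash skull pickup.
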(event OnComponentBeginOverlap(Box)
  (params (OverlappedComponent :type Primitive%20Component%20Object%20Reference) (OtherActor :type Actor%20Object%20Reference) (OtherComp :type Primitive%20Component%20Object%20Reference) (OtherBodyIndex :type Integer) (bFromSweep :type Boolean) (SweepResult :type Hit%20Result%20Structure%20%28by%20ref%29))
  (bind _escape (Variables|Default|GetEscape))
  (bind _returnvalue (Spline|GetSplineLength _escape))
  (Utilities|Casting|CastToBP_GliffPlayer OtherActor)
  (bind _newtrack_0 (Timeline|FlightTimeline Play)
    (:Update
      (Transformation|SetWorldTransform (Variables|Default|GetBird) (Math|Transform|MakeTransform (Spline|GetLocationatDistanceAlongSpline _escape (* _returnvalue _newtrack_0) "World") (Spline|GetRotationatDistanceAlongSpline _escape _returnvalue "World")) false false))))

(event OnComponentBeginOverlap(hitcolider)
  (params (OverlappedComponent :type Primitive%20Component%20Object%20Reference) (OtherActor :type Actor%20Object%20Reference) (OtherComp :type Primitive%20Component%20Object%20Reference) (OtherBodyIndex :type Integer) (bFromSweep :type Boolean) (SweepResult :type Hit%20Result%20Structure%20%28by%20ref%29))
  (bind _ns_explosion (Variables|Default|GetNS_Explosion))
  (Components|Activation|Activate _ns_explosion true)
  (Rendering|SetVisibility _ns_explosion true false)
  (Rendering|SetVisibility (Variables|Default|GetPointLight) true false)
  (Utilities|Casting|CastToBP_InHandWeapon OtherActor)
  (Collision|SetCollisionEnabled (Variables|Default|GetBox) "NoCollision")
  (Components|Activation|Deactivate (Variables|Default|GetProjectileMovement))
  (Audio|Components|Audio|Stop (Variables|Default|GetFlightTimeline))
  (Physics|SetSimulatePhysics (Variables|Default|GetBird) true)
  (Physics|SetEnableGravity (Variables|Default|GetBird) true)
  (Transformation|DetachFromComponent (Variables|Default|GetBird) "KeepWorld" "KeepWorld" "KeepWorld" false)
  (Physics|AddImpulse (Variables|Default|GetBird) "0.000000,0.000000,-1000.000000" "None" true)
  (Animation|Montage|PlayMontage (Variables|Default|GetBird) "/Game/GliffGame/Characters/Bird/AM_Birds_Anim.AM_Birds_Anim"
    (:then
      (Utilities|FlowControl|Delay 0.5)
      (CallFunction|AnyDamage))))

(event Custom|BirdDeath
  (bind _ns_explosion (Variables|Default|GetNS_Explosion))
  (Components|Activation|Activate _ns_explosion true)
  (Rendering|SetVisibility _ns_explosion true false)
  (Rendering|SetVisibility (Variables|Default|GetPointLight) true false)
  (Actor|DestroyActor)
  (bind _asbp_gliff_player (Utilities|Casting|CastToBP_GliffPlayer (Game|GetPlayerCharacter 0)))
  (Default|BullApplyHealth _asbp_gliff_player)
  (Utilities|FlowControl|Delay 0.5))

(event Custom|AnyDamage
  (Default|TookDamage (Variables|Default|GetBP_HealthSystem_Component) 0 2e+01)
  (if (<= (Variables|/Game/GliffGame/SideScrollGame/Components/BP_HealthSystem_Component.BP_HealthSystem_Component_C|GetHealth (Variables|Default|GetBP_HealthSystem_Component)) 0.0)
    (CallFunction|BirdDeath)))

(event Custom|SpawnPickUp
  ;[0.15 0.15 0.15 0.5] SpawnPickUp
  (if (not (Variables|Default|GetSkull%20Has%20Spawned))
    (bind _asbp_stash (Utilities|Casting|CastToBP_StashClass "/Game/GliffGame/PickUps/HeartGlass/BP_Stash.BP_Stash_C"))
    (bind _returnvalue (Game|SpawnActorfromClass _asbp_stash (Transformation|GetActorTransform) "Undefined" "MultiplyWithRoot" 0 0))
    (Physics|SetEnableGravity (Variables|/Game/GliffGame/PickUps/HeartGlass/BP_Stash.BP_Stash_C|GetSkull _returnvalue) true)
    (Physics|SetSimulatePhysics (Variables|/Game/GliffGame/PickUps/HeartGlass/BP_Stash.BP_Stash_C|GetSkull _returnvalue) true)
    (Physics|AddImpulse (Variables|/Game/GliffGame/PickUps/HeartGlass/BP_Stash.BP_Stash_C|GetSkull _returnvalue) "0.000000,0.000000,1000.000000" "None" true)
    (Variables|Default|SetSkull%20Has%20Spawned true)))

(fn ConstructionScript)