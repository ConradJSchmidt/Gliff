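; BP_Woman is a hazard character whose mesh yaw is animated by a timeline and which punishes the player on contact.
; An overlap plays a poof sound and explosion effect, then knocks BP_GliffPlayer along X with temporary capsule physics and a hit montage.
; When the montage completes, physics turns off and HealthStash drops to its remainder below ten.
; Each ten lost spawns a physics-driven BP_Stash skull pickup scattered near the player.
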(event OnComponentBeginOverlap(WomanCollider)
  (params (OverlappedComponent :type Primitive%20Component%20Object%20Reference) (OtherActor :type Actor%20Object%20Reference) (OtherComp :type Primitive%20Component%20Object%20Reference) (OtherBodyIndex :type Integer) (bFromSweep :type Boolean) (SweepResult :type Hit%20Result%20Structure%20%28by%20ref%29))
  (Audio|PlaySoundatLocation "/Game/GliffGame/Audio/SFX/DEAD_COW_POOF.DEAD_COW_POOF" "0, 0, 0" "0, 0, 0" 1.0 1.0 0.0 0 0 0 0)
  (Rendering|SetVisibility (Variables|Default|GetNS_Explosion) true false)
  (Components|Activation|Activate (Variables|Default|GetNS_Explosion) true)
  (bind _asbp_gliff_player (Utilities|Casting|CastToBP_GliffPlayer OtherActor))
  (Physics|SetSimulatePhysics (Variables|/Script/Engine.Character|GetCapsuleComponent _asbp_gliff_player) true)
  ;[0.15 0.15 0.15 0.5] SteelStash
  (Physics|AddImpulse (Variables|/Script/Engine.Character|GetCapsuleComponent _asbp_gliff_player) (* (Math|Vector|Normalize (- (Transformation|GetActorLocation) (Transformation|GetActorLocation _asbp_gliff_player))) "-2000.000000,0.000000,0.000000") "None" true)
  (Animation|Montage|PlayMontage (Variables|/Script/Engine.Character|GetMesh _asbp_gliff_player) "/Game/GliffGame/Characters/GliffPiggme/Animation/Eagle/06/am_TakeHit_001.am_TakeHit_001"
    (:then
      (Utilities|FlowControl|Delay 0.5)
      (Components|Activation|Deactivate (Variables|Default|GetNS_Explosion)))
    (:OnCompleted
      (Physics|SetSimulatePhysics (Variables|/Script/Engine.Character|GetCapsuleComponent _asbp_gliff_player) false)
      (if (>= (Variables|/Game/GliffGame/SideScrollGame/BP_GliffPlayer.BP_GliffPlayer_C|GetHealthStash _asbp_gliff_player) 10)
        (bind _output_get (Variables|Default|SetPickUpsToDrop (/ (Variables|/Game/GliffGame/SideScrollGame/BP_GliffPlayer.BP_GliffPlayer_C|GetHealthStash _asbp_gliff_player) 10)))
        (Variables|/Game/GliffGame/SideScrollGame/BP_GliffPlayer.BP_GliffPlayer_C|SetHealthStash _asbp_gliff_player (- (Variables|/Game/GliffGame/SideScrollGame/BP_GliffPlayer.BP_GliffPlayer_C|GetHealthStash _asbp_gliff_player) (* _output_get 10)))
        (CallFunction|SpawnPickUps)))))

(event Custom|PlayRotation
  (bind _newtrack_0 (Timeline|Timeline Play)
    (:Update
      (Transformation|SetRelativeLocationAndRotation (Variables|Default|GetWoman) "0, 0, 0" (Math|Rotator|MakeRotator 0.0 -1.0 _newtrack_0) false false))))

(event Custom|SpawnPickUps
  ;[0.15 0.15 0.15 0.5] SpawnPickUp
  (if (> (Variables|Default|GetPickUpsToDrop) 0)
    (for _index (range 0 (- (Variables|Default|GetPickUpsToDrop) 1))
      (bind _asbp_stash (Utilities|Casting|CastToBP_StashClass "/Game/GliffGame/VFX/SM/BP_Stash.BP_Stash_C"))
      (bind _returnvalue (Game|SpawnActorfromClass _asbp_stash (Math|Transform|MakeTransform (+ (Transformation|GetActorLocation (Game|Player|GetPlayerPawn 0)) (Math|Vector|MakeVector (Math|Random|RandomFloatinRange -1e+03 1e+03) 0.0 (Math|Random|RandomFloatinRange 1e+02 1.5e+02)))) "Undefined" "MultiplyWithRoot" 0 0))
      (Physics|SetEnableGravity (Variables|/Game/GliffGame/VFX/SM/BP_Stash.BP_Stash_C|GetSkull _returnvalue) true)
      (Physics|SetSimulatePhysics (Variables|/Game/GliffGame/VFX/SM/BP_Stash.BP_Stash_C|GetSkull _returnvalue) true)
      (Physics|AddImpulse (Variables|/Game/GliffGame/VFX/SM/BP_Stash.BP_Stash_C|GetSkull _returnvalue) (Math|Vector|MakeVector (Math|Random|RandomFloatinRange 1e+04 1e+04) 0.0 (Math|Random|RandomFloatinRange 5e+02 1e+03)) "None" true))))

(event EventBeginPlay
  (CallFunction|PlayRotation))

(fn ConstructionScript)