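; BP_HunterShaman is a Hunter Shaman NPC Blueprint that drives a level sequence based on player proximity.
; When a BP_GliffPlayer begins overlapping its SequenceTrigger component, it plays the sequence through the referenced LevelSequenceActor's player.
; When the player leaves the trigger, StopLevelSequence calls Play and then immediately Stop on that same sequence player.
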(event OnComponentBeginOverlap(sequenceTrigger)
  (params (OverlappedComponent :type Primitive%20Component%20Object%20Reference) (OtherActor :type Actor%20Object%20Reference) (OtherComp :type Primitive%20Component%20Object%20Reference) (OtherBodyIndex :type Integer) (bFromSweep :type Boolean) (SweepResult :type Hit%20Result%20Structure%20%28by%20ref%29))
  (Utilities|Casting|CastToBP_GliffPlayer OtherActor)
  (CallFunction|PlayLevelsSequence))

(event OnComponentEndOverlap(sequenceTrigger)
  (params (OverlappedComponent :type Primitive%20Component%20Object%20Reference) (OtherActor :type Actor%20Object%20Reference) (OtherComp :type Primitive%20Component%20Object%20Reference) (OtherBodyIndex :type Integer))
  (Utilities|Casting|CastToBP_GliffPlayer OtherActor)
  (CallFunction|StopLevelSequence))

(event Custom|PlayLevelsSequence
  (Sequencer|Player|Play (Variables|/Script/LevelSequence.LevelSequenceActor|GetSequencePlayer (Variables|Default|GetLevelSequenceActorRef)) :!class /Script/MovieScene.MovieSceneSequencePlayer))

(event Custom|StopLevelSequence
  (bind _levelsequenceactorref (Variables|Default|GetLevelSequenceActorRef))
  (bind _sequenceplayer (Variables|/Script/LevelSequence.LevelSequenceActor|GetSequencePlayer _levelsequenceactorref))
  (Sequencer|Player|Play _sequenceplayer :!class /Script/MovieScene.MovieSceneSequencePlayer)
  (Sequencer|Player|Stop _sequenceplayer :!class /Script/MovieScene.MovieSceneSequencePlayer))

(fn ConstructionScript)