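; Bee swarm controller that makes registered bees follow the player's BP_GliffPlayer pawn as a loose flock.
; AddBee and RemoveBee maintain the member list, which a looping timer processes each SwarmTick.
; Bees within SeparationDist of the player get movement input blending leader follow with cohesion toward the previous tick's computed center.
; Separation and alignment terms are present but never affect movement, as their results are overwritten or unused.
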(event Custom|SwarmTick
  (Variables|Default|SetValidBeeCount 0.0)
  (Variables|Default|SetSwarmCenterSum "0, 0, 0")
  (Variables|Default|SetSeparationForce "0, 0, 0")
  (Variables|Default|SetAlignmentSumVector "0, 0, 0")
  (Variables|Default|SetLocalSumVector "0, 0, 0")
  (for _array_element (Variables|Default|GetSwarmMembers)
    (Utilities|IsValid _array_element
      (:Is%20Valid
        (if (!= _array_element (Variables|Default|GetBeeRef))
          (Variables|Default|SetBeeRef _array_element)
          (Variables|Default|SetValidBeeCount (+ (Variables|Default|GetValidBeeCount) 1.0))
          (if (<= (Math|Vector|VectorLength (- (Transformation|GetActorLocation (Variables|Default|GetSwarmLeader)) (Transformation|GetActorLocation (Variables|Default|GetBeeRef)))) (Variables|Default|GetSeparationDist))
            (Variables|Default|SetSwarmCenterSum (+ (Variables|Default|GetSwarmCenterSum) (Transformation|GetActorLocation (Variables|Default|GetBeeRef))))
            (Variables|Default|SetLocalSumVector (+ (Variables|Default|GetLocalSumVector) (* (Math|Vector|Normalize (- (Variables|Default|GetSetSwarmCenter) (Transformation|GetActorLocation (Variables|Default|GetBeeRef)))) (Variables|Default|GetCohesionStrength))))
            (Variables|Default|SetLocalSumVector (+ (Variables|Default|GetLocalSumVector) (* (Math|Vector|Normalize (- (Transformation|GetActorLocation (Variables|Default|GetSwarmLeader)) (Transformation|GetActorLocation (Variables|Default|GetBeeRef)))) (Variables|Default|GetSeparationStrength))))
            (if (<= (Math|Vector|VectorLength (- (Transformation|GetActorLocation (Variables|Default|GetSwarmLeader)) (Transformation|GetActorLocation (Variables|Default|GetBeeRef)))) 1e+03)
              (Variables|Default|SetLocalSumVector (+ (Variables|Default|GetLocalSumVector) (* (Math|Vector|Normalize (- (Transformation|GetActorLocation (Variables|Default|GetSwarmLeader)) (Transformation|GetActorLocation (Variables|Default|GetBeeRef)))) (Variables|Default|GetFollowStrength)))))
            (Variables|Default|SetLocalSumVector (* (Math|Vector|Normalize (- (Transformation|GetActorLocation (Variables|Default|GetSwarmLeader)) (Transformation|GetActorLocation (Variables|Default|GetBeeRef)))) (Variables|Default|GetFollowStrength)))
            (Variables|Default|SetLocalSumVector (+ (Variables|Default|GetLocalSumVector) (* (Math|Vector|Normalize (- (Variables|Default|GetSetSwarmCenter) (Transformation|GetActorLocation (Variables|Default|GetBeeRef)))) (Variables|Default|GetCohesionStrength))))
            (Pawn|Input|AddMovementInput (Variables|Default|GetBeeRef) (Math|Vector|ClampVectorSize (Math|Vector|Normalize (Variables|Default|GetLocalSumVector)) 0.0 (Variables|Default|GetSwarmForceLimit)) 1.0 false)
            (Variables|Default|SetBeeRef 0))))))
  (if (> (Variables|Default|GetValidBeeCount) 0.0)
    (Variables|Default|SetSetSwarmCenter (/ (Variables|Default|GetSwarmCenterSum) (Variables|Default|GetValidBeeCount)))
    (Variables|Default|SetLocalSumVector (+ (Variables|Default|GetLocalSumVector) (* (Math|Vector|Normalize (Variables|Default|GetAlignmentSumVector)) (Variables|Default|GetAlignmentStrength))))))

(event Custom|AddBee
  (params (BeeRef :type BP%20BEES%20Object%20Reference))
  (bind _swarmmembers (Variables|Default|GetSwarmMembers))
  (if (not (Utilities|Array|ContainsItem _swarmmembers BeeRef))
    (Utilities|Array|Add _swarmmembers BeeRef)))

(event Custom|RemoveBee
  (params (BeeRef :type BP%20BEES%20Object%20Reference))
  (Utilities|IsValid BeeRef
    (:Is%20Valid
      (if (Utilities|Array|ContainsItem (Variables|Default|GetSwarmMembers) BeeRef)
        (Utilities|Array|RemoveItem (Variables|Default|GetSwarmMembers) BeeRef)))))

(event EventBeginPlay
  (bind _asbp_gliff_player (Utilities|Casting|CastToBP_GliffPlayer (Game|Player|GetPlayerPawn 0)))
  (Variables|Default|SetSwarmLeader _asbp_gliff_player)
  (Utilities|Time|SetTimerbyFunctionName 0 "SwarmTick" (Variables|Default|GetSwarmTickRate) true))

(fn ConstructionScript)