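; Dog enemy character that follows the player pawn via AI MoveTo, reissuing the move shortly after each success or failure.
; DogKilled hides the mesh, spawns Niagara, flashes two lights, plays sounds at world origin and destroys the actor, setting its guard flag only after the delays.
; DeathFX shows a burst mesh whose dynamic material animation is timed from game time.
; Camera-facing rotation for that mesh is left unconnected.
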(event Custom|DogKilled
  (if (not (Variables|Default|GetDogIsKilled))
    (CallFunction|DeathFX)
    (AddComponent|AddNiagaraComponent false)
    (Audio|PlaySoundatLocation "/Game/GliffGame/Audio/SFX/DEAD_COW_POOF_Cue.DEAD_COW_POOF_Cue" "0, 0, 0" "0, 0, 0" 1.0 1.0 0.0 0 0 0 0)
    (Rendering|SetVisibility (Variables|Default|GetPointLightDR) true false)
    (Rendering|SetVisibility (Variables|Character|GetMesh) false false)
    (Utilities|FlowControl|Delay 0.2)
    (Rendering|SetVisibility (Variables|Default|GetPointLightDR) false false)
    (Utilities|FlowControl|Delay 1.0)
    (Variables|Default|SetDogIsKilled true)
    (Actor|DestroyActor)))

(event Custom|DeathFX
  (bind _dynamic_material (Variables|Default|GetDynamic%20Material))
  (Audio|PlaySoundatLocation "/Game/GliffGame/Audio/SFX/ANIMALS_EXPLODE_FROM_LASER_GUN_4_Cue.ANIMALS_EXPLODE_FROM_LASER_GUN_4_Cue" "0, 0, 0" "0, 0, 0" 1.0 1.0 0.0 0 0 0 0)
  (Rendering|Material|SetMaterial (Variables|Default|GetSM_BurstA) 0 _dynamic_material)
  (Rendering|Material|SetScalarParameterValue _dynamic_material "AnimationControl" (Utilities|Time|GetGameTimeinSeconds) :!class /Script/Engine.MaterialInstanceDynamic)
  (Rendering|SetVisibility (Variables|Default|GetPointLightDR) true false)
  (Utilities|FlowControl|Delay 1.5)
  (Actor|DestroyActor))

(event EventBeginPlay
  (AI|AIMoveTo self "0, 0, 0" (Game|Player|GetPlayerPawn 0) 3e+02 false :!label _label
    (:OnSuccess
      _)
    (:OnFail
      _))
  (Utilities|FlowControl|Delay 0.2)
  (goto _label))

(fn ConstructionScript)