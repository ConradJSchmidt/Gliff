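; Player controller for the Gliff side-scroller that owns the player's UI and level-level input.
; On BeginPlay it creates the player info and main UI widgets, adds the default Enhanced Input context, and passes the main UI to the player pawn's health component.
; Input actions forward level reload and respawn to the game mode.
; A Win event shows the win screen and disables pawn input.
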(event Custom|Win
  (bind _returnvalue (UserInterface|CreateWidget "/Game/GliffGame/SideScrollGame/UI/WBP_WinScreen.WBP_WinScreen_C" self))
  (UserInterface|Viewport|AddtoViewport _returnvalue 0)
  (Input|DisableInput (Game|Player|GetPlayerPawn 0) self))

(event Custom|NotifyUIReady
  (bind _asbp_gliff_player (Utilities|Casting|CastToBP_GliffPlayer (Game|Player|GetPlayerPawn 0)))
  (Default|OnUiReady (Variables|/Game/GliffGame/SideScrollGame/BP_GliffPlayer.BP_GliffPlayer_C|GetBP_HealthSystem_Component _asbp_gliff_player) (Variables|Default|GetWB_UI_Ref)))

(event Input|EnhancedActionEvents|EnhancedInputActionIA_ReloadLevel
  (params (ActionValue :type Boolean) (ElapsedSeconds :type Float%20%28double-precision%29) (TriggeredSeconds :type Float%20%28double-precision%29) (InputAction :type Input%20Action%20Object%20Reference :default "/Game/GliffGame/SideScrollGame/Input/Actions/IA_ReloadLevel.IA_ReloadLevel"))
  (bind _asbp_gliff_game_mode (Utilities|Casting|CastToBP_Gliff_GameMode (Game|GetGameMode)))
  (Default|ReloadLevel _asbp_gliff_game_mode))

(event Input|EnhancedActionEvents|EnhancedInputActionIA_Respawn
  (params (ActionValue :type Boolean) (ElapsedSeconds :type Float%20%28double-precision%29) (TriggeredSeconds :type Float%20%28double-precision%29) (InputAction :type Input%20Action%20Object%20Reference :default "/Game/GliffGame/SideScrollGame/Input/Actions/IA_Respawn.IA_Respawn"))
  (bind _asbp_gliff_game_mode (Utilities|Casting|CastToBP_Gliff_GameMode (Game|GetGameMode)))
  (Default|ReSpawnPlayer _asbp_gliff_game_mode))

(event EventBeginPlay
  (bind _returnvalue (UserInterface|CreateWidget "/Game/GliffGame/SideScrollGame/UI/WBP_Playerinfo.WBP_Playerinfo_C" self))
  (bind _output_get (Variables|Default|SetPlayerInfoUiRef _returnvalue))
  (UserInterface|Viewport|AddtoViewport _output_get 0)
  (Input|AddMappingContext (PlayerController|LocalPlayerSubsystems|GetEnhancedInputLocalPlayerSubsystem self) "/Game/GliffGame/SideScrollGame/Input/IMC_Default.IMC_Default" 0 "(bIgnoreAllPressedKeysUntilRelease=True,bForceImmediately=False,bNotifyUserSettings=False)")
  (Utilities|IsValid (Variables|Default|GetWB_UI_Ref)
    (:Is%20Not%20Valid
      (bind _returnvalue_2 (UserInterface|CreateWidget "/Game/GliffGame/SideScrollGame/HUD/WB_UI.WB_UI_C" self))
      (bind _output_get_2 (Variables|Default|SetWB_UI_Ref _returnvalue_2))
      (CallFunction|NotifyUIReady)
      (UserInterface|Viewport|AddtoViewport _output_get_2 0))))

(fn ConstructionScript)