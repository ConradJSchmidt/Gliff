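; Player state for the Gliff side-scroll game that holds the player's spawn point and food stash.
; BeginPlay saves the first player pawn's transform as the spawn point.
; HandleConsumeFood spends one unit of food and flags a starvation clock update, or reports failure and a kill when the stash holds less than one unit.
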(event EventBeginPlay
  (Variables|Default|SetSpawnPoint (Transformation|GetActorTransform (Game|Player|GetPlayerPawn 0))))

(fn ConstructionScript)

(fn HandleConsumeFood
  (if (>= (Variables|Default|GetFoodStash) 1.0)
    (Variables|Default|SetFoodStash (- (Variables|Default|GetFoodStash) 1.0))
    (return true 1.0 true false)
    (else
      (return false 0.0 false true))))