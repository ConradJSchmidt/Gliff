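; BP_SplashRadial is a short-lived splash burst effect shown on the SMBurstA mesh.
; On BeginPlay it creates a dynamic M_FlipBurstA material, sets AnimationControl to zero once and makes the mesh visible.
; It turns the mesh once toward the player camera, with pitch zeroed and a 90-degree yaw offset, as a one-shot upright billboard.
; The actor destroys itself after a one-second delay.
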(event EventBeginPlay
  (bind _returnvalue (Game|GetPlayerCameraManager 0))
  (bind _animationcontrol (Variables|Default|GetAnimationControl))
  (bind _sm_bursta (Variables|Default|GetSM_BurstA))
  (bind _returnvalue_2 (Transformation|GetWorldLocation _sm_bursta))
  (bind _returnvalue_3 (Camera|GetCameraLocation _returnvalue))
  (bind _returnvalue_4 (Math|Rotator|FindLookatRotation _returnvalue_2 _returnvalue_3))
  (bind _returnvalue_5 (Rendering|Material|CreateDynamicMaterialInstance (Variables|Default|GetSM_BurstA) 0 "/Game/GliffGame/VFX/Materials/SPRITES/M_FlipBurstA.M_FlipBurstA" _animationcontrol :!class /Script/Engine.PrimitiveComponent))
  (Variables|Default|SetDynamicMaterial _returnvalue_5)
  (Rendering|Material|SetScalarParameterValue 0 _animationcontrol 0.0 :!class /Script/Engine.KismetMaterialLibrary)
  (Rendering|SetVisibility (Variables|Default|GetSM_BurstA) true false)
  (Transformation|SetWorldRotation (Variables|Default|GetSM_BurstA) (Math|Rotator|CombineRotators (Math|Rotator|MakeRotator (.roll _returnvalue_4) 0.0 (.yaw _returnvalue_4)) (Math|Rotator|MakeRotator 0.0 0.0 9e+01)) false false)
  (Utilities|FlowControl|Delay 1.0)
  (Actor|DestroyActor))

(fn ConstructionScript)