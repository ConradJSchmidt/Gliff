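; BP_BushB is an environment bush Blueprint with no active logic of its own.
; Its construction script only calls the parent's.
; The event graph holds unconnected, never-run billboard code that would yaw the Mountain component toward the player camera with a 90-degree offset, keeping pitch at zero.
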(fn ConstructionScript
  (|CallParentFunction))