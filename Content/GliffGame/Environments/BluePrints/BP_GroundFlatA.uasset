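; BP_GroundFlatA is a ground piece that procedurally covers its static mesh with grass in the construction script.
; It clears a hierarchical instanced mesh component, then loops on GrassDensity, picking random points across the ground mesh bounds at twice the Z extent.
; Each point gets two local-space instances with random per-axis scale, the mesh's roll and pitch, and random yaw ranged by its world X and Y position.
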(event EventBeginPlay)

(event Collision|EventActorBeginOverlap
  (params (OtherActor :type Actor%20Object%20Reference)))

(event EventTick
  (params (DeltaSeconds :type Float%20%28single-precision%29)))

(fn ConstructionScript
  (bind _staticmeshcomponent (Variables|Debug|GetStaticMeshComponent))
  (bind _staticmeshcomponent_2 (Variables|Debug|GetStaticMeshComponent))
  (bind _grassscalemax (Variables|Default|GetGrassScaleMax))
  (bind _grassscalemin (Variables|Default|GetGrassScaleMin))
  (bind _returnvalue (Math|Random|RandomFloatinRange _grassscalemin _grassscalemax))
  (bind _boxextent (Collision|GetComponentBounds _staticmeshcomponent))
  (bind _returnvalue_2 (Transformation|GetWorldLocation _staticmeshcomponent_2))
  (bind _returnvalue_3 (Transformation|GetWorldRotation _staticmeshcomponent_2))
  (bind (_x _y _z) (Math|Vector|BreakVector _boxextent))
  (bind (_roll _pitch) (Math|Rotator|BreakRotator _returnvalue_3))
  (bind (_x_2 _y_2) (Math|Vector|BreakVector _returnvalue_2))
  (Components|InstancedStaticMesh|ClearInstances (Variables|Default|GetHierarchicalInstancedStaticMeshGrass))
  (for _index (range 0 (Variables|Default|GetGrassDensity))
    (Variables|Default|SetRandomLocation (Math|Vector|MakeVector (Math|Random|RandomFloatinRange (* -1.0 _x) _x) (Math|Random|RandomFloatinRange (* -1.0 _y) _y) (* 2.0 _z)))
    (Components|InstancedStaticMesh|AddInstance (Variables|Default|GetHierarchicalInstancedStaticMeshGrass) (Math|Transform|MakeTransform (Variables|Default|GetRandomLocation) (Math|Rotator|MakeRotator _roll _pitch (Math|Random|RandomFloatinRange _x_2 _y_2)) (Math|Vector|MakeVector _returnvalue _returnvalue _returnvalue)) false)
    (Components|InstancedStaticMesh|AddInstance (Variables|Default|GetHierarchicalInstancedStaticMeshGrass) (Math|Transform|MakeTransform (Variables|Default|GetRandomLocation) (Math|Rotator|MakeRotator _roll _pitch (Math|Random|RandomFloatinRange _x_2 _y_2)) (Math|Vector|MakeVector _returnvalue _returnvalue _returnvalue)) false)))