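; BP_BushADark is an environment Blueprint, by its name a dark bush variant, with a component named Mountain.
; Its event graph holds billboard logic that would yaw Mountain toward the player camera with a 90-degree offset and zero pitch.
; That logic is not connected to any event, so it never runs.
; The construction script only calls its parent.
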(fn ConstructionScript
  (|CallParentFunction))