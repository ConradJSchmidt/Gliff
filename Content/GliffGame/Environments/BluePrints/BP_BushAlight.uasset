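; BP_BushAlight is an environment Blueprint with logic to turn its Mountain component toward the player camera, billboard style.
; The rotation takes yaw and roll from a look-at toward camera 0, zeroes pitch and combines in a 90-degree yaw offset.
; That logic is not wired to any event, so it never runs.
; The construction script only calls its parent.
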(fn ConstructionScript
  (|CallParentFunction))