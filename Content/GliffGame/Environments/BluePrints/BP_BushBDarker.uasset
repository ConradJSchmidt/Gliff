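; BP_BushBDarker is an environment Blueprint, by its name a darker bush variant, with a component named Mountain.
; Its event graph holds billboard logic that would turn Mountain toward the player camera with zero pitch and a 90-degree yaw offset.
; That logic is disconnected and never runs, and the construction script only calls its parent.
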(fn ConstructionScript
  (|CallParentFunction))