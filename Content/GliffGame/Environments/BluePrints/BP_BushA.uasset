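; BP_BushA is an environment Blueprint with a component named Mountain, apparently copied from a billboard-style setup.
; Its only logic would turn Mountain toward the player camera on yaw, keeping look-at roll, zeroing pitch and adding a 90-degree yaw offset.
; That rotation chain is not connected to any event, so it never runs.
; The construction script only calls its parent.
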(fn ConstructionScript
  (|CallParentFunction))