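; BP_TreeZen is an environment actor whose Mountain component turns to face the player camera, acting as an upright billboard.
; Each Tick it computes a look-at rotation from Mountain to the first player's camera and zeroes the pitch so it does not tilt toward the viewer.
; A fixed quarter-turn yaw offset is combined in before the world rotation is set.
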(event EventTick
  (params (DeltaSeconds :type Float%20%28single-precision%29))
  (bind _returnvalue (Game|GetPlayerCameraManager 0))
  (bind _mountain (Variables|Default|GetMountain))
  (bind _returnvalue_2 (Transformation|GetWorldLocation _mountain))
  (bind _returnvalue_3 (Camera|GetCameraLocation _returnvalue))
  (bind _returnvalue_4 (Math|Rotator|FindLookatRotation _returnvalue_2 _returnvalue_3))
  (Transformation|SetWorldRotation (Variables|Default|GetMountain) (Math|Rotator|CombineRotators (Math|Rotator|MakeRotator (.roll _returnvalue_4) 0.0 (.yaw _returnvalue_4)) (Math|Rotator|MakeRotator 0.0 0.0 9e+01)) false false))

(fn ConstructionScript
  (|CallParentFunction))