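; Sprint ability component for the side-scroll game that switches movement between walking and sprinting speed.
; StartSprint and StopSprint take a CharacterMovement reference and set its MaxWalkSpeed to SprintSpeed or WalkSpeed.
; An IsSprinting flag guards both functions, so each change applies only when the sprint state actually flips.
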(fn StartSprint
  (params (Character%20Movement :type Character%20Movement%20Component%20Object%20Reference))
  (if (not (Variables|Default|GetIsSprinting))
    (Variables|Default|SetIsSprinting true)
    (Variables|/Script/Engine.CharacterMovementComponent|SetMaxWalkSpeed Character%20Movement (Variables|Default|GetSprintSpeed))))

(fn StopSprint
  (params (CharacterMovement :type Character%20Movement%20Component%20Object%20Reference))
  (if (Variables|Default|GetIsSprinting)
    (Variables|Default|SetIsSprinting false)
    (Variables|/Script/Engine.CharacterMovementComponent|SetMaxWalkSpeed CharacterMovement (Variables|Default|GetWalkSpeed))))