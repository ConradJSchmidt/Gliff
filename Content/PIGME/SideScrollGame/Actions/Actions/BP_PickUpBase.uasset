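; Base pickup actor for a side-scrolling game, providing the shared collect behavior.
; A sphere overlap plays optional sound and Niagara burst effects at the actor's location, calls PickUp with player pawn 0, then destroys the actor.
; PickUp here only prints a debug string, serving as a placeholder.
; The player-pawn comparison is left unconnected, so any overlapping actor triggers collection.
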(event OnComponentBeginOverlap(Sphere)
  (params (OverlappedComponent :type Primitive%20Component%20Object%20Reference) (OtherActor :type Actor%20Object%20Reference) (OtherComp :type Primitive%20Component%20Object%20Reference) (OtherBodyIndex :type Integer) (bFromSweep :type Boolean) (SweepResult :type Hit%20Result%20Structure%20%28by%20ref%29))
  (if true
    (CallFunction|PlayFX)
    (CallFunction|PickUp (Game|Player|GetPlayerPawn 0))
    (Actor|DestroyActor)))

(event Custom|PickUp
  (params (PlayerPawn :type Pawn%20Object%20Reference))
  (Development|PrintString "BasePickUp"))

(fn ConstructionScript)

(fn PlayFX
  (bind _pickupsound (Variables|BaseFX|GetPickUpSound))
  (bind _pickupparticleburst (Variables|Default|GetPickUpParticleBurst))
  (Utilities|IsValid _pickupsound
    (:Is%20Valid
      (Audio|PlaySoundatLocation _pickupsound (Transformation|GetActorLocation) "0, 0, 0" 1.0 1.0 0.0 0 0 0 0))
    (:Is%20Not%20Valid
      _))
  (Utilities|IsValid _pickupparticleburst
    (:Is%20Valid
      (Niagara|SpawnSystematLocation _pickupparticleburst (Transformation|GetActorLocation)))
    (:Is%20Not%20Valid
      _))
  (return))