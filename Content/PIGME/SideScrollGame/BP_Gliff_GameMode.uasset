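; BP_Gliff_GameMode is a game mode for the Gliff side-scroller that handles winning, level reload and player respawn.
; The Win event forwards to the first player's BP_Gliff_PlayerControler.
; ReloadLevel reopens the current level by name.
; ReSpawnPlayer destroys any valid controlled pawn, then restarts the player at the SpawnPoint transform stored in BP_GliffPlayerState.
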(event Custom|Win
  (bind _asbp_gliff_player_controler (Utilities|Casting|CastToBP_Gliff_PlayerControler (Game|GetPlayerController 0)))
  (Default|Win _asbp_gliff_player_controler))

(event EventBeginPlay)

(event EventTick
  (params (DeltaSeconds :type Float%20%28single-precision%29)))

(fn ConstructionScript)

(fn ReloadLevel
  (bind _returnvalue (Game|GetCurrentLevelName true))
  (Game|OpenLevel(byName) (Utilities|String|StringToName _returnvalue)))

(fn ReSpawnPlayer
  (bind _returnvalue (Game|GetPlayerController 0))
  (bind _returnvalue_2 (Pawn|GetControlledPawn _returnvalue))
  (if (Utilities|IsValid _returnvalue_2)
    (Actor|DestroyActor _returnvalue_2))
  (bind _asbp_gliff_player_state (Utilities|Casting|CastToBP_GliffPlayerState (Game|GetPlayerState 0)))
  (Class|GameModeBase|RestartPlayeratTransform (Game|GetPlayerController 0) (Variables|/Game/PIGME/SideScrollGame/BP_GliffPlayerState.BP_GliffPlayerState_C|GetSpawnPoint _asbp_gliff_player_state)))