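; BP_CaveMan is a caveman enemy that attacks the player, BP_GliffPlayer, with a club.
; Two strike trigger volumes each play the club-strike montage on its mesh when the player begins overlapping them, with a debug print.
; A damage collider applies fixed damage when it hits the player and plays a take-hit montage on player 0's mesh, with an empty branch on completion.
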(event OnComponentBeginOverlap(StrikeTrigger)
  (params (OverlappedComponent :type Primitive%20Component%20Object%20Reference) (OtherActor :type Actor%20Object%20Reference) (OtherComp :type Primitive%20Component%20Object%20Reference) (OtherBodyIndex :type Integer) (bFromSweep :type Boolean) (SweepResult :type Hit%20Result%20Structure%20%28by%20ref%29))
  (Utilities|Casting|CastToBP_GliffPlayer OtherActor)
  (Development|PrintString "MontageTriggered")
  (Animation|Montage|PlayMontage (Variables|Character|GetMesh) "/Game/PIGME/Characters/CaveMan/AM_CaveManStrikeClub.AM_CaveManStrikeClub"))

(event OnComponentBeginOverlap(StrikeTrigger1)
  (params (OverlappedComponent :type Primitive%20Component%20Object%20Reference) (OtherActor :type Actor%20Object%20Reference) (OtherComp :type Primitive%20Component%20Object%20Reference) (OtherBodyIndex :type Integer) (bFromSweep :type Boolean) (SweepResult :type Hit%20Result%20Structure%20%28by%20ref%29))
  (Utilities|Casting|CastToBP_GliffPlayer OtherActor)
  (Development|PrintString "MontageTriggered")
  (Animation|Montage|PlayMontage (Variables|Character|GetMesh) "/Game/PIGME/Characters/CaveMan/AM_CaveManStrikeClub.AM_CaveManStrikeClub"))

(event OnComponentHit(DamageColider)
  (params (HitComponent :type Primitive%20Component%20Object%20Reference) (OtherActor :type Actor%20Object%20Reference) (OtherComp :type Primitive%20Component%20Object%20Reference) (NormalImpulse :type Vector :default "0, 0, 0") (Hit :type Hit%20Result%20Structure%20%28by%20ref%29))
  (bind _asbp_gliff_player (Utilities|Casting|CastToBP_GliffPlayer OtherActor))
  (Game|Damage|ApplyDamage _asbp_gliff_player 1e+01 0 0)
  (Animation|Montage|PlayMontage (Variables|/Script/Engine.Character|GetMesh (Game|GetPlayerCharacter 0)) "/Game/PIGME/Characters/GliffPiggme/Animation/Eagle/06/am_TakeHit_001.am_TakeHit_001"
    (:OnCompleted
      (if true
        _))))

(event EventBeginPlay)

(event Collision|EventActorBeginOverlap
  (params (OtherActor :type Actor%20Object%20Reference)))

(event EventTick
  (params (DeltaSeconds :type Float%20%28single-precision%29)))

(fn ConstructionScript)