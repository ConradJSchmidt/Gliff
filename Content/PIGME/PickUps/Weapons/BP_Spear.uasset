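; BP_Spear is a throwable spear weapon that damages BP_Bulls when its tip overlaps one, then destroys itself.
; On Thrown, it constrains projectile movement to a plane if the BP_GliffPlayer is in side-scroll mode, otherwise frees it.
; It then plays a sound, enables physics, derives velocity from pawn and weapon motion along the pawn's forward vector, swaps the in-hand mesh for the spear mesh, and activates projectile movement.
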(event OnComponentBeginOverlap(spearTip)
  (params (OverlappedComponent :type Primitive%20Component%20Object%20Reference) (OtherActor :type Actor%20Object%20Reference) (OtherComp :type Primitive%20Component%20Object%20Reference) (OtherBodyIndex :type Integer) (bFromSweep :type Boolean) (SweepResult :type Hit%20Result%20Structure%20%28by%20ref%29))
  (bind _asbp_bulls (Utilities|Casting|CastToBP_Bulls OtherActor))
  (Game|Damage|ApplyDamage _asbp_bulls 25.0 0 0)
  (Actor|DestroyActor))

(event EventThrown
  (bind _projectilemovement (Variables|Default|GetProjectileMovement))
  (bind _projectilemovement_2 (Variables|Default|GetProjectileMovement))
  (bind _asbp_gliff_player (Utilities|Casting|CastToBP_GliffPlayer (Game|GetPlayerCharacter 0)))
  (if (Variables|/Game/PIGME/SideScrollGame/BP_GliffPlayer.BP_GliffPlayer_C|GetIsSideScroll _asbp_gliff_player)
    (Class|MovementComponent|SetPlaneConstraintEnabled _projectilemovement_2 true)
    (Class|MovementComponent|SetPlaneConstraintNormal _projectilemovement_2 "0.000000,1.000000,0.000000")
    (else
      (Development|PrintString "IsThirdPerson")
      (Class|MovementComponent|SetPlaneConstraintEnabled _projectilemovement false)
      (Class|MovementComponent|SetPlaneConstraintNormal _projectilemovement "0, 0, 0")))
  (Audio|PlaySoundatLocation (Variables|Default|GetSoundWeapon) "0, 0, 0" "0, 0, 0" 1.0 1.0 0.0 0 0 0 0)
  (Physics|SetSimulatePhysics (Variables|Default|GetSM_Spear) true)
  (Game|Components|ProjectileMovement|SetVelocityinLocalSpace (Variables|Default|GetProjectileMovement) (* (+ (Transformation|GetVelocity (Game|Player|GetPlayerPawn 0)) (Transformation|GetComponentVelocity (Variables|Default|GetWeaponComponent))) (Transformation|GetActorForwardVector (Game|Player|GetPlayerPawn 0))))
  (Rendering|SetVisibility (Variables|Default|GetInHandWeapon) false false)
  (Rendering|SetVisibility (Variables|Default|GetSM_Spear) true false)
  (Components|Activation|Activate (Variables|Default|GetProjectileMovement) false))

(fn ConstructionScript)