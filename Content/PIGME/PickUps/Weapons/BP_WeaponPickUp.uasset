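; Weapon pickup that equips a data-table weapon on an overlapping BP_GliffPlayer.
; BeginPlay starts a yaw timeline for the mesh, sets the mesh from a table row named None, and creates a burst material instance.
; Overlap looks up WeaponRowNames, passes that row to EquipWeapon, then plays sound and a time-stamped flipbook burst with light before destroying itself.
; The camera-facing burst rotation is never executed.
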(event OnComponentBeginOverlap(PickUpCollision)
  (params (OverlappedComponent :type Primitive%20Component%20Object%20Reference) (OtherActor :type Actor%20Object%20Reference) (OtherComp :type Primitive%20Component%20Object%20Reference) (OtherBodyIndex :type Integer) (bFromSweep :type Boolean) (SweepResult :type Hit%20Result%20Structure%20%28by%20ref%29))
  ;[0.15 0.15 0.15 0.5] OnPick Up
  (bind _asbp_gliff_player (Utilities|Casting|CastToBP_GliffPlayer OtherActor))
  (bind _output_get (Variables|Default|SetWeaponRowNames (Variables|Default|GetWeaponRowNames)))
  (bind _returnvalue (Utilities|GetDataTableRow (Variables|Default|GetWeaponDataTable) _output_get)
    (:then
      (Utilities|Array|Add (Variables|/Game/PIGME/SideScrollGame/BP_GliffPlayer.BP_GliffPlayer_C|GetPlayerInventory _asbp_gliff_player) "")
      (Default|EquipWeapon _asbp_gliff_player 0 (.Damage (Utilities|Struct|BreakBP_WeaponData _returnvalue)) (.FireRate (Utilities|Struct|BreakBP_WeaponData _returnvalue)) (.WeaponMesh (Utilities|Struct|BreakBP_WeaponData _returnvalue)) (.ThrownWeaponClass (Utilities|Struct|BreakBP_WeaponData _returnvalue)) (.AmmoCount (Utilities|Struct|BreakBP_WeaponData _returnvalue)) "NewEnumerator0")
      (CallFunction|TriggerFX))
    (:RowNotFound
      (Development|PrintString "Fail"))))

(event Custom|TriggerFX
  ;[0.15 0.15 0.15 0.5] TriggerFX
  (Audio|PlaySoundatLocation (Variables|Default|GetPickUpSound) "0, 0, 0" "0, 0, 0" 1.0 1.0 0.0 0 0 0 0)
  (Rendering|Material|SetMaterial (Variables|Default|GetSM_BurstA) 0 (Variables|Default|GetDynamicMaterial))
  (Rendering|Material|SetScalarParameterValue (Variables|Default|GetDynamicMaterial) "AnimationControl" (Utilities|Time|GetGameTimeinSeconds) :!class /Script/Engine.MaterialInstanceDynamic)
  (Rendering|SetVisibility (Variables|Default|GetSM_BurstA) true false)
  (Rendering|SetVisibility (Variables|Default|GetDefaultSceneRoot) false false)
  (Collision|SetCollisionEnabled (Variables|Default|GetPickUpCollision) "NoCollision")
  (Utilities|FlowControl|Delay 1.0)
  (Actor|DestroyActor))

(event EventBeginPlay
  ;[0.15 0.15 0.15 0.5] SetWeapons
  (Utilities|FlowControl|Sequence
    (:then_0
      (bind _newtrack_0 (Timeline|Timeline Play)
        (:Update
          (Transformation|SetRelativeLocationAndRotation (Variables|Default|GetWeaponMesh) "0, 0, 0" (Math|Rotator|MakeRotator 0.0 -1.0 _newtrack_0) false false))))
    (:then_1
      (bind _returnvalue (Utilities|GetDataTableRow (Variables|Default|GetWeaponDataTable) "")
        (:then
          (Components|StaticMesh|SetStaticMesh (Variables|Default|GetWeaponMesh) (.WeaponMesh (Utilities|Struct|BreakBP_WeaponData _returnvalue))))))
    (:then_2
      (bind _returnvalue_2 (Rendering|Material|CreateDynamicMaterialInstance (Variables|Default|GetSM_BurstA) 0 "/Game/PIGME/VFX/Materials/SPRITES/M_FlipBurstA.M_FlipBurstA" "None" :!class /Script/Engine.PrimitiveComponent))
      (Variables|Default|SetDynamicMaterial _returnvalue_2))))

(fn ConstructionScript)