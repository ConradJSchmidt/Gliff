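; BP_Food is a food pickup that adds to the player's HealthStash when touched.
; A sphere overlap with BP_GliffPlayer adds a fixed amount to the stash, prints the new value, destroys the pickup and calls the player's CheckHealthStash.
; On BeginPlay, a timeline drives the yaw of the SmRootLeaf component at a raised, fixed relative height to animate the pickup.
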(event OnComponentBeginOverlap(Sphere1)
  (params (OverlappedComponent :type Primitive%20Component%20Object%20Reference) (OtherActor :type Actor%20Object%20Reference) (OtherComp :type Primitive%20Component%20Object%20Reference) (OtherBodyIndex :type Integer) (bFromSweep :type Boolean) (SweepResult :type Hit%20Result%20Structure%20%28by%20ref%29))
  (bind _asbp_gliff_player (Utilities|Casting|CastToBP_GliffPlayer OtherActor))
  (bind _output_get (Variables|/Game/PIGME/SideScrollGame/BP_GliffPlayer.BP_GliffPlayer_C|SetHealthStash _asbp_gliff_player (+ (Variables|/Game/PIGME/SideScrollGame/BP_GliffPlayer.BP_GliffPlayer_C|GetHealthStash _asbp_gliff_player) 20)))
  (Development|PrintString (Utilities|String|ToString(Integer) _output_get))
  (Actor|DestroyActor)
  (Default|CheckHealthStash _asbp_gliff_player))

(event Collision|EventActorBeginOverlap
  (params (OtherActor :type Actor%20Object%20Reference)))

(event EventTick
  (params (DeltaSeconds :type Float%20%28single-precision%29)))

(event EventBeginPlay
  (bind _newtrack_0 (Timeline|Timeline PlayFromStart)
    (:Update
      (Transformation|SetRelativeLocationAndRotation (Variables|Default|Getsm_rootLeaf) "0.000000,0.000000,100.000000" (Math|Rotator|MakeRotator 0.0 0.0 _newtrack_0) false false))))

(fn ConstructionScript)