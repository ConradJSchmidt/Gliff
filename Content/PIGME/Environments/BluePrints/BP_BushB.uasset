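; BP_BushB is an environment Blueprint, named as a bush, with a component called Mountain.
; Its Event Graph holds billboard logic that would yaw Mountain toward the player camera with a 90-degree offset, using a look-at rotation with zeroed pitch.
; That logic is not connected to any event, so it never runs.
; The Construction Script only calls its parent.
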(fn ConstructionScript
  (|CallParentFunction))