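; BP_BushA is an environment Blueprint for a bush, with a component named Mountain.
; Its event graph holds unconnected billboard logic that would rotate Mountain toward the player camera, zeroing pitch and adding a 90-degree yaw offset.
; That logic never runs, and the construction script only calls its parent, so the Blueprint's graphs add no behavior.
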(fn ConstructionScript
  (|CallParentFunction))