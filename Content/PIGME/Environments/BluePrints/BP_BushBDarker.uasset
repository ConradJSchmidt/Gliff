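; BP_BushBDarker is an environment child Blueprint, by its name a darker bush variant, with no active logic of its own.
; Its construction script only calls the parent's.
; The event graph holds disconnected billboard code that never runs: it would turn the Mountain component toward the player camera, zeroing pitch and adding a yaw offset.
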(fn ConstructionScript
  (|CallParentFunction))