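; BP_BushAlight is an environment Blueprint whose only authored logic is an unused billboard rotation for its Mountain component.
; That disconnected logic would turn Mountain toward player 0's camera, keeping look-at yaw and roll, zeroing pitch and adding a 90-degree yaw offset.
; No event triggers it, and the construction script only calls its parent, so this Blueprint's graphs add no behavior.
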(fn ConstructionScript
  (|CallParentFunction))