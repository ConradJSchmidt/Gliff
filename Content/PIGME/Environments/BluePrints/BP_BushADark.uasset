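; BP_BushADark is an environment Blueprint, named as a dark bush, with a component called Mountain.
; Its Event Graph holds unconnected billboard logic that would yaw Mountain toward the player camera, with zero pitch and a 90-degree yaw offset.
; No event runs that logic, and the Construction Script only calls its parent, so the graphs add no active behavior.
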(fn ConstructionScript
  (|CallParentFunction))