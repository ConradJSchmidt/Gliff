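; BP_FireTrap is a fire trap that warms up when triggered, then turns hot and destroys any Character that begins overlapping its damage volume.
; An enum-style state machine cycles Idle, Warming and Hot through ChangeState, which runs exit and enter functions.
; The activation volume fires OnTrapTouch, bound only while Idle, and timers advance the later states.
; Enter and exit functions switch particles, audio and damage collision, and print debug strings.
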(event OnComponentBeginOverlap(ActivateVolume)
  (params (OverlappedComponent :type Primitive%20Component%20Object%20Reference) (OtherActor :type Actor%20Object%20Reference) (OtherComp :type Primitive%20Component%20Object%20Reference) (OtherBodyIndex :type Integer) (bFromSweep :type Boolean) (SweepResult :type Hit%20Result%20Structure%20%28by%20ref%29))
  (Default|CallOnTrapTouch))

(event OnComponentBeginOverlap(DamageVolume)
  (params (OverlappedComponent :type Primitive%20Component%20Object%20Reference) (OtherActor :type Actor%20Object%20Reference) (OtherComp :type Primitive%20Component%20Object%20Reference) (OtherBodyIndex :type Integer) (bFromSweep :type Boolean) (SweepResult :type Hit%20Result%20Structure%20%28by%20ref%29))
  (bind _ascharacter (Utilities|Casting|CastToCharacter OtherActor))
  (Actor|DestroyActor _ascharacter))

(event EventTick
  (params (DeltaSeconds :type Float%20%28single-precision%29))
  (switch Utilities|FlowControl|Switch|SwitchonE_FireTrapState (Variables|Default|GetCurrentState)))

(event EventBeginPlay
  (Collision|SetCollisionEnabled (Variables|Default|GetDamageVolume) "NoCollision")
  (CallFunction|ChangeState "NewEnumerator0"))

(fn ConstructionScript)

(fn ChangeState
  (params (NewState :type E_FireTrapState%20Enum :default "NewEnumerator0"))
  (if (Variables|Default|GetIsInitialState)
    (Variables|Default|SetIsInitialState false)
    (Variables|Default|SetCurrentState NewState :!label _label)
    (switch Utilities|FlowControl|Switch|SwitchonE_FireTrapState (Variables|Default|GetCurrentState)
      (:NewEnumerator0
        (IdleState|EnterIdleState))
      (:NewEnumerator1
        (WarmingState|EnterWarmingState))
      (:NewEnumerator2
        (HotState|EnterHotState)))
    (elif (not (Utilities|Enum|Equal(Enum) NewState (Variables|Default|GetCurrentState)))
      (switch Utilities|FlowControl|Switch|SwitchonE_FireTrapState (Variables|Default|GetCurrentState)
        (:NewEnumerator0
          (IdleState|ExitIdleState)
          (goto _label))
        (:NewEnumerator1
          (WarmingState|ExitWarmingState)
          (goto _label))
        (:NewEnumerator2
          (HotState|ExitHotState)
          (goto _label))))))

(fn EnterIdleState
  (Development|PrintString "EnterIdleState" true true "(R=0.018210,G=0.442708,B=0.000000,A=1.000000)")
  (EventDispatchers|BindEventtoOnTrapTouch (EventDispatchers|CreateEvent :!event ActivateTrap)))

(fn TickIdleState)

(fn ExitIdleState
  (Development|PrintString "ExitIdleState")
  (EventDispatchers|UnbindEventfromOnTrapTouch (EventDispatchers|CreateEvent :!event ActivateTrap)))

(fn ActivateTrap
  (CallFunction|ChangeState "NewEnumerator1"))

(fn ExitWarmingState
  (Development|PrintString "ExitWarmingState")
  (Components|Activation|Deactivate (Variables|Default|GetTrapParticles)))

(fn EnterWarmingState
  (bind _trapparticles (Variables|Default|GetTrapParticles))
  (Development|PrintString "EnterWarmingState")
  (Class|NiagaraComponent|SetAsset _trapparticles (Variables|WarmingState|GetWarmingParticles) true)
  (Components|Activation|Activate _trapparticles false)
  (Audio|PlaySoundatLocation (Variables|WarmingState|GetActivateWarmingSound) (Transformation|GetActorLocation) "0, 0, 0" 1.0 1.0 0.0 0 0 0 0)
  (Utilities|Time|SetTimerbyFunctionName 0 "OnWarmingTimerEnded" (Variables|WarmingState|GetWarmingDuration)))

(fn TickWarmingState)

(fn EnterHotState
  (bind _trapparticles (Variables|Default|GetTrapParticles))
  (bind _trapaudio (Variables|Default|GetTrapAudio))
  (Development|PrintString "EnterHotState")
  (Collision|SetCollisionEnabled (Variables|Default|GetDamageVolume) "QueryAndPhysics")
  (Class|NiagaraComponent|SetAsset _trapparticles (Variables|HotState|GetHotParticles) true)
  (Components|Activation|Activate _trapparticles false)
  (Audio|Components|Audio|SetSound _trapaudio (Variables|HotState|GetHotLoopingSound))
  (Components|Activation|Activate _trapaudio false)
  (Audio|PlaySoundatLocation (Variables|HotState|GetHotActivateSound) (Transformation|GetActorLocation) "0, 0, 0" 1.0 1.0 0.0 0 0 0 0)
  (Utilities|Time|SetTimerbyFunctionName 0 "OnHotTimerEnded" (Variables|HotState|GetHotDuration)))

(fn ExitHotState
  (Development|PrintString "ExitHotState")
  (Collision|SetCollisionEnabled (Variables|Default|GetDamageVolume) "NoCollision")
  (Components|Activation|Deactivate (Variables|Default|GetTrapParticles))
  (Components|Activation|Deactivate (Variables|Default|GetTrapAudio)))

(fn TickHotState)

(fn OnWarmingTimerEnded
  (CallFunction|ChangeState "NewEnumerator2"))

(fn OnHotTimerEnded
  (CallFunction|ChangeState "NewEnumerator0"))